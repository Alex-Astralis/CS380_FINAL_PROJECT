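; Spawner actor that creates a stack or row of Box_BP actors one at a time after play begins.
; A looping timer started on BeginPlay spawns each box at the spawner's transform, shifted by Offset times the current count, until BoxesToSpawn is reached.
; Spawned boxes are stored in BoxArray, which GetNextBox exposes by index.
; The timer is never cleared, so it keeps firing after the limit.
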(event Custom|StartTimer
  (bind _returnvalue (Transformation|GetActorTransform))
  (if (< (Variables|Default|GetCounter) (Variables|Default|GetBoxesToSpawn))
    (bind _returnvalue_2 (Game|SpawnActorfromClass "/Game/Blueprints/Box_BP.Box_BP_C" (Math|Transform|MakeTransform (+ (.location _returnvalue) (* (Variables|Default|Getoffset) (Variables|Default|GetCounter))) (.rotation _returnvalue) (.scale _returnvalue)) "Undefined" 0 0))
    (Utilities|Array|Add (Variables|Default|GetBoxArray) _returnvalue_2)
    (bind _result (Math|Integer|IncrementInt (Variables|Default|GetCounter))
      (:%20%20
        (Variables|Default|SetCounter _result)))))

(event EventBeginPlay
  (bind _returnvalue (Utilities|Time|SetTimerbyEvent (delegate Custom|StartTimer) (Variables|Default|GetDelay) true))
  (Variables|Default|SetTimer _returnvalue))

(event Collision|EventActorBeginOverlap
  (params (OtherActor :type Actor%20Object%20Reference)))

(event EventTick
  (params (DeltaSeconds :type Float%20%28single-precision%29)))

(fn ConstructionScript)

(fn GetNextBox
  (params (Index :type Integer))
  (bind _output_get (Variables|Default|SetBoxBuffer (Utilities|Array|Get(acopy) (Variables|Default|GetBoxArray) Index)))
  (return _output_get))