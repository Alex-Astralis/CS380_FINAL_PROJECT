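; AI controller for the Grabber, which runs its behavior tree and seeds the blackboard with the player reference.
; GetNewBox asks the Grabber's spawner for the box at the current index and stores it as the blackboard target.
; Each tick sets an in-range flag from the pawn's distance to that box, clearing it when no valid box exists.
; DestroyBox destroys the box and advances the index.
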(event Custom|RangeCheck
  (bind _next_box (Variables|Default|GetNext%20Box))
  (bind _blackboard (Variables|Default|GetBlackboard))
  (bind _key_inrange (Variables|Default|GetKey_InRange))
  (Utilities|IsValid _next_box
    (:Is%20Valid
      (if (<= (Math|Vector|Distance(Vector) (Transformation|GetActorLocation _next_box) (Transformation|GetActorLocation (Pawn|GetControlledPawn))) 1e+02)
        (AI|Components|Blackboard|SetValueasBool _blackboard _key_inrange true)
        (else
          (AI|Components|Blackboard|SetValueasBool _blackboard _key_inrange false :!label _label))))
    (:Is%20Not%20Valid
      (goto _label))))

(event EventBeginPlay
  (bind _blackboardcomponent (Class|AIController|UseBlackboard "/Game/BehaviorTree/Blackboards/Grabber_Blackboard.Grabber_Blackboard"))
  (AI|Components|Blackboard|SetValueasObject _blackboardcomponent (Variables|Default|GetKey_PlayerRef) (Game|GetPlayerCharacter 0))
  (AI|RunBehaviorTree "/Game/BehaviorTree/BT_Grabber.BT_Grabber"))

(event EventTick
  (params (DeltaSeconds :type Float%20%28single-precision%29))
  (CallFunction|RangeCheck))

(fn ConstructionScript)

(fn GetNewBox
  (bind _asgrabber (Utilities|Casting|CastToGrabber (AI|Components|Blackboard|GetValueasObject (Variables|Default|GetBlackboard) (Variables|Default|GetKey_SelfActor))))
  (bind _nextbox (Default|GetNextBox (Variables|/Game/Blueprints/Grabber.Grabber_C|GetSpawnerRef _asgrabber) (Variables|Default|GetIndex)))
  (Variables|Default|SetNext%20Box _nextbox)
  (AI|Components|Blackboard|SetValueasObject (Variables|Default|GetBlackboard) (Variables|Default|GetKey_BoxRef) _nextbox)
  (Development|PrintString (Utilities|GetDisplayName _nextbox)))

(fn DestroyBox
  (bind _next_box (Variables|Default|GetNext%20Box))
  (Utilities|IsValid _next_box
    (:Is%20Valid
      (Actor|DestroyActor _next_box)
      (bind _result (Math|Integer|IncrementInt (Variables|Default|GetIndex))
        (:%20%20
          (bind _output_get (Variables|Default|SetIndex _result))
          (Development|PrintString (Utilities|String|ToString(Integer) _output_get)))))))