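; AI controller that drives a pawn through a sequence of spawned boxes using the BT_TouchBox behavior tree and BB_TouchBox blackboard.
; GetNewBox pulls the indexed box from the Grabber's spawner into the blackboard; DestroyBox and ChangeBox act on it and advance the index.
; Tick flags whether an untouched box is within range.
; Events push a new behavior tree or pop back after a short delay.
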(event Custom|SwitchToNewBehavior
  (params (Next%20Behavior%20Tree :type Behavior%20Tree%20Object%20Reference))
  (Class|MyAIController|PushBehaviorTree Next%20Behavior%20Tree))

(event Custom|PopOldBehavior
  (Utilities|FlowControl|Delay 1.0)
  (Class|MyAIController|PopBehaviorTree))

(event EventTick
  (params (DeltaSeconds :type Float%20%28single-precision%29))
  (bind _next_box (Variables|Default|GetNext%20Box))
  (bind _blackboard (Variables|Default|GetBlackboard))
  (bind _key_inrange (Variables|Default|GetKey_InRange))
  (Utilities|IsValid _next_box
    (:Is%20Valid
      (if (<= (Math|Vector|Distance(Vector) (Transformation|GetActorLocation _next_box) (Transformation|GetActorLocation (Pawn|GetControlledPawn))) 2e+02)
        (if (Variables|/Game/Blueprints/Box_BP.Box_BP_C|GetBTouched _next_box)
          (AI|Components|Blackboard|SetValueasBool _blackboard _key_inrange false :!label _label)
          (else
            (AI|Components|Blackboard|SetValueasBool _blackboard _key_inrange true)))
        (else
          (goto _label))))
    (:Is%20Not%20Valid
      (goto _label))))

(fn ConstructionScript)

(fn GetNewBox
  (bind _asgrabber (Utilities|Casting|CastToGrabber (AI|Components|Blackboard|GetValueasObject (Variables|Default|GetBlackboard) (Variables|Default|GetKey_SelfActor))))
  (bind _nextbox (Default|GetNextBox (Variables|/Game/Blueprints/Grabber.Grabber_C|GetSpawnerRef _asgrabber) (Variables|Default|GetIndex)))
  (Variables|Default|SetNext%20Box _nextbox)
  (AI|Components|Blackboard|SetValueasObject (Variables|Default|GetBlackboard) (Variables|Default|GetKey_BoxRef) _nextbox)
  (Development|PrintString (Utilities|GetDisplayName _nextbox)))

(fn DestroyBox
  (bind _next_box (Variables|Default|GetNext%20Box))
  (Utilities|IsValid _next_box
    (:Is%20Valid
      (Actor|DestroyActor _next_box)
      (bind _result (Math|Integer|IncrementInt (Variables|Default|GetIndex))
        (:%20%20
          (bind _output_get (Variables|Default|SetIndex _result))
          (Development|PrintString (Utilities|String|ToString(Integer) _output_get)))))))

(fn ChangeBox
  (Utilities|IsValid (Variables|Default|GetNext%20Box)
    (:Is%20Valid
      (if (not (Variables|/Game/Blueprints/Box_BP.Box_BP_C|GetBTouched (Variables|Default|GetNext%20Box)))
        (Default|ChangeBoxEvent (Variables|Default|GetNext%20Box))
        (bind _result (Math|Integer|IncrementInt (Variables|Default|GetIndex))
          (:%20%20
            (bind _output_get (Variables|Default|SetIndex _result))
            (Development|PrintString (Utilities|String|ToString(Integer) _output_get))
            (bind _output_get_2 (Variables|Default|SetNext%20Box 0))
            (AI|Components|Blackboard|SetValueasObject (Variables|Default|GetBlackboard) (Variables|Default|GetKey_BoxRef) _output_get_2)))))))

(event EventBeginPlay
  (bind _blackboardcomponent (Class|AIController|UseBlackboard "/Game/BehaviorTree/Blackboards/BB_TouchBox.BB_TouchBox"))
  (AI|Components|Blackboard|SetValueasObject _blackboardcomponent (Variables|Default|GetKey_PlayerRef) (Game|GetPlayerCharacter 0))
  (Class|MyAIController|SetBehaviorTree "/Game/BehaviorTree/BT_TouchBox.BT_TouchBox")
  (AI|RunBehaviorTree "/Game/BehaviorTree/BT_TouchBox.BT_TouchBox"))